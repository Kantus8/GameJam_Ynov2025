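; BP_Ressource is a resource pickup that adds its amount to the player's HUD total when touched by an attached BP_Bubble.
; On spawn, Sphere1 gets a random-strength impulse roughly toward the player, using a randomly yawed look-at rotation.
; Collection spawns a RadialBurst effect and destroys the actor.
; Uncollected pickups periodically check whether they were recently rendered and destroy themselves once off screen.
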(event OnComponentBeginOverlap(Sphere)
  (params (OverlappedComponent :type Primitive%20Component%20Object%20Reference) (OtherActor :type Actor%20Object%20Reference) (OtherComp :type Primitive%20Component%20Object%20Reference) (OtherBodyIndex :type Integer) (bFromSweep :type Boolean) (SweepResult :type Hit%20Result%20Structure%20%28by%20ref%29))
  (bind _bpplayer (Variables|Default|GetBPplayer))
  (bind _hud (Variables|/Game/BP/BP_Player.BP_Player_C|GetHUD _bpplayer))
  (bind _asbp_bubble (Utilities|Casting|CastToBP_Bubble OtherActor))
  (if (Variables|/Game/BP/BP_Bubble.BP_Bubble_C|GetAttached _asbp_bubble)
    (Variables|/Game/BubbleGame/WB_HUD.WB_HUD_C|SetRessources _hud (+ (Variables|/Game/BubbleGame/WB_HUD.WB_HUD_C|GetRessources _hud) (Variables|Default|GetRessourceAmount)))
    (Niagara|SpawnSystematLocation "/Niagara/DefaultAssets/Templates/Systems/RadialBurst.RadialBurst" (Transformation|GetWorldLocation (Variables|Default|GetSphere1)) "0, 0, 0" "0.700000,0.700000,0.700000")
    (Actor|DestroyActor)))

(event EventBeginPlay
  (bind _returnvalue (Actor|GetActorOfClass "/Game/BP/BP_Player.BP_Player_C"))
  (bind _output_get (Variables|Default|SetBPplayer _returnvalue))
  (Physics|AddImpulse (Variables|Default|GetSphere1) (* (Math|Vector|GetRightVector (Math|Rotator|CombineRotators (Math|Rotator|FindLookatRotation (Transformation|GetActorLocation) (Transformation|GetActorLocation _output_get)) (Math|Rotator|MakeRotator 0.0 0.0 (Math|Random|RandomFloatinRange -135.0 -45.0)))) (Math|Random|RandomFloatinRange 1e+01 175.0)) "None" true)
  (Utilities|FlowControl|RetriggerableDelay 15.0 :!label _label)
  (if (Class|Actor|WasRecentlyRendered 0.2)
    (goto _label)
    (else
      (Actor|DestroyActor))))

(fn ConstructionScript)