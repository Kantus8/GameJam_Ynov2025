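; Spawner actor for the bubble game that periodically scatters BP_Ressource pickups around itself.
; A looping timer started on BeginPlay fires SpawnRessource, which spawns a random batch of zero to three resources.
; Each lands on a random navigable point within a fixed radius of the Sphere component, at a fixed height, always spawning with collision adjustment when possible.
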(event Custom|SpawnRessource
  (bind _sphere (Variables|Default|GetSphere))
  (bind _returnvalue (Transformation|GetWorldLocation _sphere))
  (Variables|Default|SetNumberOfSpawns (Math|Random|RandomInteger 4))
  (while (>= (Variables|Default|GetNumberOfSpawns) 1)
    (bind _randomlocation (Class|NavigationSystemV1|GetRandomLocationinNavigableRadius (Math|Vector|MakeVector (.x _returnvalue) (.y _returnvalue) 5e+01) 5e+02 0 0))
    (Game|SpawnActorfromClass "/Game/BubbleGame/BP_Ressource.BP_Ressource_C" (Math|Transform|MakeTransform (Math|Vector|MakeVector (.x _randomlocation) (.y _randomlocation) 5e+01) "0, 0, 0" "1.000000,1.000000,1.000000") "AdjustIfPossibleButAlwaysSpawn" "MultiplyWithRoot" 0 0)
    (Math|Integer|DecrementInt (Variables|Default|GetNumberOfSpawns))))

(event EventBeginPlay
  (Utilities|Time|SetTimerbyEvent (delegate Custom|SpawnRessource) 5.0 true))

(fn ConstructionScript)