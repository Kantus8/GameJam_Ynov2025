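; Background bubble spawner for the bubble game, judging by its name, that periodically spawns actors around its Sphere component.
; A looping timer started on BeginPlay fires SpawnRessource, which rolls a random count of zero or one and loops to spawn that many.
; Each spawn gets a random horizontal offset from the sphere and a random negative world height, adjusting for collisions but always spawning.
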(event Custom|SpawnRessource
  (bind _sphere (Variables|Default|GetSphere))
  (bind _returnvalue (Transformation|GetWorldLocation _sphere))
  (Variables|Default|SetNumberOfSpawns (Math|Random|RandomInteger 2))
  (while (>= (Variables|Default|GetNumberOfSpawns) 1)
    (Game|SpawnActorfromClass "/Game/BubbleGame/BP_BackgroundBubble.BP_BackgroundBubble_C" (Math|Transform|MakeTransform (Math|Vector|MakeVector (+ (.x _returnvalue) (Math|Random|RandomFloatinRange -5e+02 5e+02)) (+ (.y _returnvalue) (Math|Random|RandomFloatinRange -5e+02 5e+02)) (Math|Random|RandomFloatinRange -5e+02 -1.5e+03)) "0, 0, 0" "1.000000,1.000000,1.000000") "AdjustIfPossibleButAlwaysSpawn" "MultiplyWithRoot" 0 0)
    (Math|Integer|DecrementInt (Variables|Default|GetNumberOfSpawns))))

(event EventBeginPlay
  (Utilities|Time|SetTimerbyEvent (delegate Custom|SpawnRessource) 1e+01 true))

(fn ConstructionScript)