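; BP_Turret is an auto-firing turret that targets BP_Enemy2 actors entering its Sphere.
; Overlapping enemies join EnemyInSight; Cube1 turns to the nearest and spawns a BP_Projectile toward it.
; A DoOnce gate and one-second cooldown loop through Reset to repeat fire.
; End overlap only prints; when the nearest enemy is outside, the loop removes the array's first entry, not necessarily that enemy, and retries while entries remain.
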(event OnComponentBeginOverlap(Sphere)
  (params (OverlappedComponent :type Primitive%20Component%20Object%20Reference) (OtherActor :type Actor%20Object%20Reference) (OtherComp :type Primitive%20Component%20Object%20Reference) (OtherBodyIndex :type Integer) (bFromSweep :type Boolean) (SweepResult :type Hit%20Result%20Structure%20%28by%20ref%29))
  (bind _enemyinsight (Variables|Default|GetEnemyInSight))
  (bind _enemyinsight_2 (Variables|Default|GetEnemyInSight))
  (bind _cube1 (Variables|Default|GetCube1))
  (bind _cube1_2 (Variables|Default|GetCube1))
  (bind _returnvalue (Transformation|GetWorldLocation _cube1_2))
  (bind _returnvalue_2 (Transformation|GetWorldLocation _cube1))
  (bind _returnvalue_3 (Actor|FindNearestActor _returnvalue _enemyinsight))
  (bind _returnvalue_4 (Transformation|GetActorLocation _returnvalue_3))
  (bind _returnvalue_5 (Math|Rotator|FindLookatRotation _returnvalue_2 _returnvalue_4))
  (bind _asbp_enemy_2 (Utilities|Casting|CastToBP_Enemy2 OtherActor))
  (Utilities|Array|AddUnique (Variables|Default|GetEnemyInSight) _asbp_enemy_2)
  (if (Collision|IsOverlappingActor (Variables|Default|GetSphere) _returnvalue_3 :!class /Script/Engine.PrimitiveComponent)
    (Utilities|FlowControl|DoOnce false
      (:Completed
        (Transformation|SetWorldRotation (Variables|Default|GetCube1) _returnvalue_5 false false)
        (Game|SpawnActorfromClass "/Game/BubbleGame/BP_Projectile.BP_Projectile_C" (Math|Transform|MakeTransform _returnvalue_2 _returnvalue_5 "1.000000,1.000000,1.000000") "Undefined" "MultiplyWithRoot" 0 0)
        (CallFunction|StartCooldown)))
    (else
      (Development|PrintString "Hello")
      (Utilities|Array|RemoveIndex _enemyinsight_2)
      (if (Utilities|Array|IsNotEmpty _enemyinsight_2)
        (CallFunction|Reset)))))

(event OnComponentEndOverlap(Sphere)
  (params (OverlappedComponent :type Primitive%20Component%20Object%20Reference) (OtherActor :type Actor%20Object%20Reference) (OtherComp :type Primitive%20Component%20Object%20Reference) (OtherBodyIndex :type Integer))
  (Utilities|Casting|CastToBP_Enemy2 OtherActor)
  (Development|PrintString "FINITO"))

(event Custom|Start%20Cooldown
  (Utilities|FlowControl|Delay 1.0)
  (CallFunction|Reset))

(event Custom|Reset
  (bind _enemyinsight (Variables|Default|GetEnemyInSight))
  (bind _enemyinsight_2 (Variables|Default|GetEnemyInSight))
  (bind _cube1 (Variables|Default|GetCube1))
  (bind _cube1_2 (Variables|Default|GetCube1))
  (bind _returnvalue (Transformation|GetWorldLocation _cube1_2))
  (bind _returnvalue_2 (Transformation|GetWorldLocation _cube1))
  (bind _returnvalue_3 (Actor|FindNearestActor _returnvalue _enemyinsight))
  (bind _returnvalue_4 (Transformation|GetActorLocation _returnvalue_3))
  (bind _returnvalue_5 (Math|Rotator|FindLookatRotation _returnvalue_2 _returnvalue_4))
  (Utilities|FlowControl|Sequence
    (:then_0
      (goto _label Reset))
    (:then_1
      (if (Collision|IsOverlappingActor (Variables|Default|GetSphere) _returnvalue_3 :!class /Script/Engine.PrimitiveComponent)
        (Utilities|FlowControl|DoOnce false :!label _label
          (:Completed
            (Transformation|SetWorldRotation (Variables|Default|GetCube1) _returnvalue_5 false false)
            (Game|SpawnActorfromClass "/Game/BubbleGame/BP_Projectile.BP_Projectile_C" (Math|Transform|MakeTransform _returnvalue_2 _returnvalue_5 "1.000000,1.000000,1.000000") "Undefined" "MultiplyWithRoot" 0 0)
            (CallFunction|StartCooldown)))
        (else
          (Development|PrintString "Hello")
          (Utilities|Array|RemoveIndex _enemyinsight_2)
          (if (Utilities|Array|IsNotEmpty _enemyinsight_2)
            (CallFunction|Reset)))))))

(fn ConstructionScript)