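; Enemy spawner for BubbleGame that places BP_Enemy2 actors at random navigable points around its Sphere component, at a fixed height.
; A looping timer fires SpawnWave, which raises MaxWaveSize each time and spawns a random count up to that cap, so waves can grow over time.
; A second looping timer spawns single enemies at an interval randomized once at BeginPlay, then held constant.
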(event Custom|SpawnWave
  (bind _result (Math|Integer|IncrementInt (Variables|Default|GetMaxWaveSize))
    (:%20%20
      (Variables|Default|SetNumberOfSpawns (Math|Random|RandomIntegerinRange 1 _result))
      (while (>= (Variables|Default|GetNumberOfSpawns) 1)
        (bind _randomlocation (Class|NavigationSystemV1|GetRandomLocationinNavigableRadius (Transformation|GetWorldLocation (Variables|Default|GetSphere)) 4e+02 0 0))
        (Game|SpawnActorfromClass "/Game/BubbleGame/BP_Enemy2.BP_Enemy2_C" (Math|Transform|MakeTransform (Math|Vector|MakeVector (.x _randomlocation) (.y _randomlocation) 55.0) "0, 0, 0" "1.000000,1.000000,1.000000") "AlwaysSpawn" "MultiplyWithRoot" 0 0)
        (Math|Integer|DecrementInt (Variables|Default|GetNumberOfSpawns))))))

(event Custom|CustomEvent
  (bind _randomlocation (Class|NavigationSystemV1|GetRandomLocationinNavigableRadius (Transformation|GetWorldLocation (Variables|Default|GetSphere)) 4e+02 0 0))
  (Game|SpawnActorfromClass "/Game/BubbleGame/BP_Enemy2.BP_Enemy2_C" (Math|Transform|MakeTransform (Math|Vector|MakeVector (.x _randomlocation) (.y _randomlocation) 55.0) "0, 0, 0" "1.000000,1.000000,1.000000") "AlwaysSpawn" "MultiplyWithRoot" 0 0))

(event EventBeginPlay
  (Utilities|Time|SetTimerbyEvent (delegate Custom|SpawnWave) 2e+01 true)
  (Utilities|Time|SetTimerbyEvent (delegate Custom|CustomEvent) (Math|Random|RandomFloatinRange 8.0 2e+01) true))

(fn ConstructionScript)