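; Bubble building block of the player's structure; loose bubbles join an attached one on hit, with a component-tag check, a sound and a scale pop.
; Each parent records its children in ActorList, forming a tree registered with BP_Player.
; BP_Enemy2 damage or a delete-mode click recursively destroys the branch, removing steers and motors from the player.
; The prime bubble survives hidden and shows the Game Over widget instead.
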(event OnComponentHit(Core)
  (params (HitComponent :type Primitive%20Component%20Object%20Reference) (OtherActor :type Actor%20Object%20Reference) (OtherComp :type Primitive%20Component%20Object%20Reference) (NormalImpulse :type Vector :default "0, 0, 0") (Hit :type Hit%20Result%20Structure%20%28by%20ref%29))
  (if (Variables|Default|GetAttached)
    (bind _asbp_bubble (Utilities|Casting|CastToBP_Bubble OtherActor))
    (Utilities|FlowControl|Delay 0.0)
    (if (Utilities|Array|Identical (Variables|/Script/Engine.ActorComponent|GetComponentTags (Variables|BP_Bubble_C|GetOther%20Comp _asbp_bubble)) (Variables|/Script/Engine.ActorComponent|GetComponentTags (Variables|Default|GetCore)))
      (Variables|BP_Bubble_C|SetOther%20Comp _asbp_bubble 0)
      (Transformation|AttachComponentToComponent (Variables|BP_Bubble_C|GetCore _asbp_bubble) (Variables|Default|GetCore) "None" "KeepWorld" "KeepWorld" "KeepWorld" true)
      (Variables|BP_Bubble_C|SetAttached _asbp_bubble true)
      (Default|AddBubble (Variables|Default|GetPlayer) (Variables|BP_Bubble_C|GetCore _asbp_bubble))
      (Audio|PlaySound2D "/Game/BubbleGame/Sons/Separation3.Separation3" 1.0 1.0 0.0 0 0)
      (CallFunction|List OtherActor)
      (CallFunction|Anim _asbp_bubble)
      (else
        (Variables|BP_Bubble_C|SetOther%20Comp _asbp_bubble 0)))
    (else
      (Variables|Default|SetOther%20Comp OtherComp))))

(event Custom|List
  (params (NewParam :type Actor%20Object%20Reference))
  (Utilities|Array|Add (Variables|Default|GetActor%20List) NewParam))

(event Custom|Kill
  (bind _player (Variables|Default|GetPlayer))
  (Variables|Default|SetAttached false)
  (Utilities|Array|RemoveItem (Variables|/Game/BP/BP_Player.BP_Player_C|GetCore (Variables|Default|GetPlayer)) (Variables|Default|GetCore))
  (for _array_element (Variables|Default|GetActor%20List)
    (bind _asbp_bubble (Utilities|Casting|CastToBP_Bubble _array_element))
    (CallFunction|Kill _asbp_bubble))
  (for _array_element_2 (Variables|Default|GetActor%20List)
    (Utilities|Casting|CastToBP_Steer _array_element_2
      (:then
        (Default|RemoveSteer _player))
      (:CastFailed
        (Utilities|Casting|CastToBP_Motor _array_element_2
          (:then
            (Default|RemoveMotor _player))
          (:CastFailed
            _))))
    (Actor|DestroyActor _array_element_2))
  (Actor|DestroyActor))

(event Custom|Anim
  (Audio|PlaySound2D "/Game/BubbleGame/Sons/Apparition-3.Apparition-3" 1.0 1.0 0.0 0 0)
  (Variables|Default|SetNewVar (Transformation|GetWorldScale (Variables|Default|GetExterior)))
  (bind _newtrack_0 (Timeline|Timeline PlayFromStart)
    (:Update
      (Transformation|SetWorldScale3D (Variables|Default|GetExterior) (* (Variables|Default|GetNewVar) (Math|Float|Lerp 1.0 1.1 _newtrack_0))))))

(event EventBeginPlay
  (Input|EnableInput (Game|GetPlayerController 0))
  (bind _returnvalue (Actor|GetActorOfClass "/Game/BP/BP_Player.BP_Player_C"))
  (Variables|Default|SetPlayer _returnvalue)
  (if (Variables|Default|GetAttached)
    (Default|AddBubble (Variables|Default|GetPlayer) (Variables|Default|GetCore))
    (Audio|PlaySound2D "/Game/BubbleGame/Sons/Apparition-3.Apparition-3" 1.0 1.0 0.0 0 0)
    (Variables|Default|SetNewVar (Transformation|GetWorldScale (Variables|Default|GetExterior)))
    (bind _newtrack_0 (Timeline|Timeline PlayFromStart)
      (:Update
        (Transformation|SetWorldScale3D (Variables|Default|GetExterior) (* (Variables|Default|GetNewVar) (Math|Float|Lerp 1.0 1.1 _newtrack_0)))))))

(event Game|Damage|EventAnyDamage
  (params (Damage :type Float%20%28single-precision%29) (DamageType :type Damage%20Type%20Object%20Reference) (InstigatedBy :type Controller%20Object%20Reference) (DamageCauser :type Actor%20Object%20Reference))
  (bind _player (Variables|Default|GetPlayer))
  (Utilities|Casting|CastToBP_Enemy2 DamageCauser)
  (if (Variables|Default|GetIs%20Prime)
    _
    (else
      (Utilities|Array|RemoveItem (Variables|/Game/BP/BP_Player.BP_Player_C|GetCore (Variables|Default|GetPlayer)) (Variables|Default|GetCore))))
  (for _array_element (Variables|Default|GetActor%20List)
    (bind _asbp_bubble (Utilities|Casting|CastToBP_Bubble _array_element)
      (:then
        (Utilities|IsValid _asbp_bubble
          (:Is%20Valid
            (CallFunction|Kill _asbp_bubble))))
      (:CastFailed
        _))
    (bind _asbp_steer (Utilities|Casting|CastToBP_Steer _array_element)
      (:then
        (Default|RemoveSteer _player)
        (Actor|DestroyActor _asbp_steer))
      (:CastFailed
        _))
    (bind _asbp_motor (Utilities|Casting|CastToBP_Motor _array_element)
      (:then
        (Default|RemoveMotor _player)
        (Actor|DestroyActor _asbp_motor))
      (:CastFailed
        (Utilities|Casting|CastToBP_Bubble _array_element
          (:CastFailed
            (Utilities|IsValid _array_element
              (:Is%20Valid
                (Actor|DestroyActor _array_element))))))))
  (Utilities|FlowControl|Delay 0.0)
  (if (Variables|Default|GetIs%20Prime)
    (Rendering|SetVisibility (Variables|Default|GetExterior) false false)
    (Viewport|RemoveAllWidgets)
    (bind _returnvalue (UserInterface|CreateWidget "/Game/BubbleGame/WB_GameOver.WB_GameOver_C"))
    (Default|INITGAMEOVER _returnvalue (Variables|Default|GetPlayer))
    (UserInterface|Viewport|AddtoViewport _returnvalue 0)
    (else
      (Niagara|SpawnSystematLocation "/Niagara/DefaultAssets/Templates/Systems/RadialBurst.RadialBurst" (Transformation|GetWorldLocation (Variables|Default|GetCore)) "0, 0, 0" "0.700000,0.700000,0.700000")
      (Actor|DestroyActor))))

(event MouseInput|EventActorOnClicked
  (params (ButtonPressed :type Key%20Structure :default "None"))
  (bind _player (Variables|Default|GetPlayer))
  (if (Variables|/Game/BP/BP_Player.BP_Player_C|GetDelete (Variables|Default|GetPlayer))
    (if (Variables|Default|GetIs%20Prime)
      _
      (else
        (Utilities|Array|RemoveItem (Variables|/Game/BP/BP_Player.BP_Player_C|GetCore (Variables|Default|GetPlayer)) (Variables|Default|GetCore))))
    (for _array_element (Variables|Default|GetActor%20List)
      (bind _asbp_bubble (Utilities|Casting|CastToBP_Bubble _array_element)
        (:then
          (Utilities|IsValid _asbp_bubble
            (:Is%20Valid
              (CallFunction|Kill _asbp_bubble))))
        (:CastFailed
          _))
      (bind _asbp_steer (Utilities|Casting|CastToBP_Steer _array_element)
        (:then
          (Default|RemoveSteer _player)
          (Actor|DestroyActor _asbp_steer))
        (:CastFailed
          _))
      (bind _asbp_motor (Utilities|Casting|CastToBP_Motor _array_element)
        (:then
          (Default|RemoveMotor _player)
          (Actor|DestroyActor _asbp_motor))
        (:CastFailed
          (Utilities|Casting|CastToBP_Bubble _array_element
            (:CastFailed
              (Utilities|IsValid _array_element
                (:Is%20Valid
                  (Actor|DestroyActor _array_element))))))))
    (Utilities|FlowControl|Delay 0.0)
    (if (Variables|Default|GetIs%20Prime)
      (Rendering|SetVisibility (Variables|Default|GetExterior) false false)
      (Viewport|RemoveAllWidgets)
      (bind _returnvalue (UserInterface|CreateWidget "/Game/BubbleGame/WB_GameOver.WB_GameOver_C"))
      (Default|INITGAMEOVER _returnvalue (Variables|Default|GetPlayer))
      (UserInterface|Viewport|AddtoViewport _returnvalue 0)
      (else
        (Niagara|SpawnSystematLocation "/Niagara/DefaultAssets/Templates/Systems/RadialBurst.RadialBurst" (Transformation|GetWorldLocation (Variables|Default|GetCore)) "0, 0, 0" "0.700000,0.700000,0.700000")
        (Actor|DestroyActor)))))

(fn ConstructionScript)