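; Placement preview for bubble attachments (motor, steer, turret, pique), with Init swapping mesh and overlap radius for all but the turret.
; Tick snaps it around the Core component nearest the deprojected cursor, facing that component.
; Sphere overlaps with motors or steers drive CanSpawn and a red/green MPC_Color tint.
; Left click spawns the part, attaches it to that component and registers it with BP_Bubble; right click cancels.
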(event OnComponentBeginOverlap(Sphere1)
  (params (OverlappedComponent :type Primitive%20Component%20Object%20Reference) (OtherActor :type Actor%20Object%20Reference) (OtherComp :type Primitive%20Component%20Object%20Reference) (OtherBodyIndex :type Integer) (bFromSweep :type Boolean) (SweepResult :type Hit%20Result%20Structure%20%28by%20ref%29))
  (bind _sphere1 (Variables|Default|GetSphere1))
  (Utilities|Casting|CastToBP_Motor OtherActor
    (:then
      _)
    (:CastFailed
      (Utilities|Casting|CastToBP_Steer OtherActor)))
  (if (or (== (Utilities|Array|Length (Collision|GetOverlappingActors _sphere1 "/Game/BP/BP_Motor.BP_Motor_C" :!class /Script/Engine.PrimitiveComponent)) 0) (== (Utilities|Array|Length (Collision|GetOverlappingActors _sphere1 "/Game/BP/BP_Steer.BP_Steer_C" :!class /Script/Engine.PrimitiveComponent)) 0))
    (Variables|Default|SetCanSpawn false)
    (Rendering|Material|SetVectorParameterValue "/Game/BP/ChaosMesh/MPC_Color.MPC_Color" "Color" (Utilities|Struct|MakeLinearColor 1.0 0.0 0.0 1.0) :!class /Script/Engine.KismetMaterialLibrary)))

(event OnComponentEndOverlap(Sphere1)
  (params (OverlappedComponent :type Primitive%20Component%20Object%20Reference) (OtherActor :type Actor%20Object%20Reference) (OtherComp :type Primitive%20Component%20Object%20Reference) (OtherBodyIndex :type Integer))
  (bind _sphere1 (Variables|Default|GetSphere1))
  (Utilities|Casting|CastToBP_Motor OtherActor
    (:then
      _)
    (:CastFailed
      (Utilities|Casting|CastToBP_Steer OtherActor)))
  (if (and (== (Utilities|Array|Length (Collision|GetOverlappingActors _sphere1 "/Game/BP/BP_Motor.BP_Motor_C" :!class /Script/Engine.PrimitiveComponent)) 0) (== (Utilities|Array|Length (Collision|GetOverlappingActors _sphere1 "/Game/BP/BP_Steer.BP_Steer_C" :!class /Script/Engine.PrimitiveComponent)) 0))
    (Variables|Default|SetCanSpawn true)
    (Rendering|Material|SetVectorParameterValue "/Game/BP/ChaosMesh/MPC_Color.MPC_Color" "Color" (Utilities|Struct|MakeLinearColor 0.0 1.0 0.0 1.0) :!class /Script/Engine.KismetMaterialLibrary)))

(event Custom|Init
  (params (NewParam :type BP%20Player%20Object%20Reference) (NewParam2 :type Actor%20Class%20Reference))
  (bind _preview (Variables|Default|GetPreview))
  (bind _sphere1 (Variables|Default|GetSphere1))
  (bind _preview_2 (Variables|Default|GetPreview))
  (Variables|Default|SetNew%20Param%202 NewParam2)
  (bind _output_get (Variables|Default|SetNew%20Param NewParam))
  (Input|EnableInput (Game|GetPlayerController 0))
  (Variables|Default|SetCore (Variables|/Game/BP/BP_Player.BP_Player_C|GetCore _output_get))
  (if (== (Variables|Default|GetNew%20Param%202) "/Game/BP/BP_Steer.BP_Steer_C")
    (Components|StaticMesh|SetStaticMesh _preview_2 "/Game/BP/ChaosMesh/Steer.Steer")
    (Components|Sphere|SetSphereRadius _sphere1 1e+01 true)
    (Transformation|SetRelativeRotation _preview "0, 0, 0" false false)
    (elif (== (Variables|Default|GetNew%20Param%202) "/Game/BP/BP_Motor.BP_Motor_C")
      (Components|StaticMesh|SetStaticMesh _preview_2 "/Game/BP/ChaosMesh/Motor.Motor")
      (Components|Sphere|SetSphereRadius _sphere1 21.0 true)
      (Transformation|SetRelativeRotation _preview "0, 0, 0" false false)
      (elif (== (Variables|Default|GetNew%20Param%202) "/Game/BP/BP_Pique.BP_Pique_C")
        (Components|StaticMesh|SetStaticMesh _preview_2 "/Game/BP/ChaosMesh/Pique.Pique")
        (Components|Sphere|SetSphereRadius _sphere1 21.0 true)
        (Transformation|SetRelativeRotation _preview "0.000000,180.000000,0.000000" false false)))))

(event EventTick
  (params (DeltaSeconds :type Float%20%28single-precision%29))
  (bind _returnvalue (Game|GetPlayerController 0))
  (bind _newvar (Variables|Default|GetNewVar))
  (bind _newvar_0 (Variables|Default|GetNewVar_0))
  (bind _worldlocation (Game|Player|ConvertMouseLocationToWorldSpace _returnvalue))
  (for _array_element (Variables|Default|GetCore)
    (Utilities|Map|Add _newvar _array_element (Math|Conversions|ToFloat(Integer) (Math|Float|Truncate (Math|Vector|Distance(Vector) (Transformation|GetWorldLocation _array_element) _worldlocation))))
    (Utilities|Map|Add _newvar_0 (Math|Conversions|ToFloat(Integer) (Math|Float|Truncate (Math|Vector|Distance(Vector) (Transformation|GetWorldLocation _array_element) _worldlocation))) _array_element))
  (bind _values (Utilities|Map|Values _newvar))
  (Transformation|SetActorLocation (Math|Vector|MakeVector (.x (+ (Transformation|GetWorldLocation (.Value (Utilities|Map|Find _newvar_0 (.MinValue (Math|Float|MinOfFloatArray _values))))) (* (Math|Vector|GetRightVector (Math|Rotator|CombineRotators (Math|Rotator|FindLookatRotation (Transformation|GetWorldLocation (.Value (Utilities|Map|Find _newvar_0 (.MinValue (Math|Float|MinOfFloatArray _values))))) _worldlocation) "0.000000,-90.000000,0.000000")) 6e+01))) (.y (+ (Transformation|GetWorldLocation (.Value (Utilities|Map|Find _newvar_0 (.MinValue (Math|Float|MinOfFloatArray _values))))) (* (Math|Vector|GetRightVector (Math|Rotator|CombineRotators (Math|Rotator|FindLookatRotation (Transformation|GetWorldLocation (.Value (Utilities|Map|Find _newvar_0 (.MinValue (Math|Float|MinOfFloatArray _values))))) _worldlocation) "0.000000,-90.000000,0.000000")) 6e+01))) 5e+01) false false)
  (Transformation|SetActorRotation (Math|Rotator|FindLookatRotation (Transformation|GetActorLocation) (Transformation|GetWorldLocation (.Value (Utilities|Map|Find _newvar_0 (.MinValue (Math|Float|MinOfFloatArray _values))))))))

(event Input|MouseEvents|LeftMouseButton
  (params (Key :type Key%20Structure :default "None"))
  (bind _returnvalue (Transformation|GetActorLocation))
  (bind _returnvalue_2 (Transformation|GetActorLocation))
  (bind _returnvalue_3 (Transformation|GetActorLocation))
  (bind _returnvalue_4 (Transformation|GetActorLocation))
  (bind _new_param_2 (Variables|Default|GetNew%20Param%202))
  (:Pressed
    (if (Variables|Default|GetCanSpawn)
      (if (== _new_param_2 "/Game/BP/BP_Motor.BP_Motor_C")
        (bind _returnvalue_5 (Game|SpawnActorfromClass "/Game/BP/BP_Motor.BP_Motor_C" (Math|Transform|MakeTransform (Math|Vector|MakeVector (.x _returnvalue_4) (.y _returnvalue_4) 5e+01) (Transformation|GetActorRotation) "1.000000,1.000000,1.000000") "Undefined" "MultiplyWithRoot" 0 0))
        (Class|BPIInit|Initialisation(Message) _returnvalue_5 (Variables|Default|GetNew%20Param))
        (Transformation|AttachComponentToComponent (Variables|/Game/BP/BP_Motor.BP_Motor_C|GetCube _returnvalue_5) (.Value (Utilities|Map|Find (Variables|Default|GetNewVar_0) (.MinValue (Math|Float|MinOfFloatArray (stale EventTick _values))))) "None" "KeepWorld" "KeepWorld" "KeepWorld" true)
        (bind _asbp_bubble (Utilities|Casting|CastToBP_Bubble (Components|GetOwner (.Value (Utilities|Map|Find (Variables|Default|GetNewVar_0) (.MinValue (Math|Float|MinOfFloatArray (stale EventTick _values))))))))
        (Default|List _asbp_bubble _returnvalue_5)
        (Actor|DestroyActor)
        (Utilities|Map|Clear (Variables|Default|GetNewVar) :!label _label)
        (Utilities|Map|Clear (Variables|Default|GetNewVar_0))
        (Default|ResetSpawnItem (Variables|Default|GetNew%20Param))
        (elif (== _new_param_2 "/Game/BP/BP_Steer.BP_Steer_C")
          (bind _returnvalue_6 (Game|SpawnActorfromClass "/Game/BP/BP_Steer.BP_Steer_C" (Math|Transform|MakeTransform (Math|Vector|MakeVector (.x _returnvalue_2) (.y _returnvalue_2) 5e+01) (Transformation|GetActorRotation) "1.000000,1.000000,1.000000") "Undefined" "MultiplyWithRoot" 0 0))
          (Class|BPIInit|Initialisation(Message) _returnvalue_6 (Variables|Default|GetNew%20Param))
          (Transformation|AttachComponentToComponent (Variables|/Game/BP/BP_Steer.BP_Steer_C|GetCube1 _returnvalue_6) (.Value (Utilities|Map|Find (Variables|Default|GetNewVar_0) (.MinValue (Math|Float|MinOfFloatArray (stale EventTick _values))))) "None" "KeepWorld" "KeepWorld" "KeepWorld" true)
          (bind _asbp_bubble_2 (Utilities|Casting|CastToBP_Bubble (Components|GetOwner (.Value (Utilities|Map|Find (Variables|Default|GetNewVar_0) (.MinValue (Math|Float|MinOfFloatArray (stale EventTick _values))))))))
          (Default|List _asbp_bubble_2 _returnvalue_6)
          (Actor|DestroyActor)
          (goto _label)
          (elif (== _new_param_2 "/Game/BubbleGame/BP_Turret.BP_Turret_C")
            (bind _returnvalue_7 (Game|SpawnActorfromClass "/Game/BubbleGame/BP_Turret.BP_Turret_C" (Math|Transform|MakeTransform (Math|Vector|MakeVector (.x _returnvalue_3) (.y _returnvalue_3) 1e+02) (Math|Rotator|CombineRotators (Transformation|GetActorRotation) "0.000000,180.000000,0.000000") "1.000000,1.000000,1.000000") "Undefined" "MultiplyWithRoot" 0 0))
            (Class|BPIInit|Initialisation(Message) _returnvalue_7 (Variables|Default|GetNew%20Param))
            (Transformation|AttachComponentToComponent (Variables|/Game/BubbleGame/BP_Turret.BP_Turret_C|GetCube1 _returnvalue_7) (.Value (Utilities|Map|Find (Variables|Default|GetNewVar_0) (.MinValue (Math|Float|MinOfFloatArray (stale EventTick _values))))) "None" "KeepWorld" "KeepWorld" "KeepWorld" true)
            (bind _asbp_bubble_3 (Utilities|Casting|CastToBP_Bubble (Components|GetOwner (.Value (Utilities|Map|Find (Variables|Default|GetNewVar_0) (.MinValue (Math|Float|MinOfFloatArray (stale EventTick _values))))))))
            (Default|List _asbp_bubble_3 _returnvalue_7)
            (Actor|DestroyActor)
            (goto _label)
            (elif (== _new_param_2 "/Game/BP/BP_Pique.BP_Pique_C")
              (bind _returnvalue_8 (Game|SpawnActorfromClass "/Game/BP/BP_Pique.BP_Pique_C" (Math|Transform|MakeTransform (Math|Vector|MakeVector (.x _returnvalue) (.y _returnvalue) 5e+01) (Math|Rotator|CombineRotators (Transformation|GetActorRotation) "0.000000,180.000000,0.000000") "1.000000,1.000000,1.000000") "Undefined" "MultiplyWithRoot" 0 0))
              (Class|BPIInit|Initialisation(Message) _returnvalue_8 (Variables|Default|GetNew%20Param))
              (Transformation|AttachComponentToComponent (Variables|/Game/BP/BP_Pique.BP_Pique_C|GetCube1 _returnvalue_8) (.Value (Utilities|Map|Find (Variables|Default|GetNewVar_0) (.MinValue (Math|Float|MinOfFloatArray (stale EventTick _values))))) "None" "KeepWorld" "KeepWorld" "KeepWorld" true)
              (bind _asbp_bubble_4 (Utilities|Casting|CastToBP_Bubble (Components|GetOwner (.Value (Utilities|Map|Find (Variables|Default|GetNewVar_0) (.MinValue (Math|Float|MinOfFloatArray (stale EventTick _values))))))))
              (Default|List _asbp_bubble_4 _returnvalue_8)
              (Actor|DestroyActor)
              (goto _label))))))))

(event Input|MouseEvents|RightMouseButton
  (params (Key :type Key%20Structure :default "None"))
  (:Pressed
    (Default|ResetSpawnItem (Variables|Default|GetNew%20Param))
    (Actor|DestroyActor)))

(fn ConstructionScript)