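; Placement preview for BP_Bubble that follows the mouse around the Core components supplied by its initializing object.
; Each Tick maps truncated cursor distances to find the nearest core, then sits at a fixed offset from it toward the cursor.
; BP_Motor or BP_Steer overlaps toggle CanSpawn and a red/green MPC_Color.
; Left-click spawns, attaches and registers a bubble; right-click cancels; both reset the initializer's spawn state and destroy the preview.
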(event OnComponentBeginOverlap(Sphere1)
  (params (OverlappedComponent :type Primitive%20Component%20Object%20Reference) (OtherActor :type Actor%20Object%20Reference) (OtherComp :type Primitive%20Component%20Object%20Reference) (OtherBodyIndex :type Integer) (bFromSweep :type Boolean) (SweepResult :type Hit%20Result%20Structure%20%28by%20ref%29))
  (bind _sphere1 (Variables|Default|GetSphere1))
  (Utilities|Casting|CastToBP_Motor OtherActor
    (:then
      _)
    (:CastFailed
      (Utilities|Casting|CastToBP_Steer OtherActor)))
  (if (or (== (Utilities|Array|Length (Collision|GetOverlappingActors _sphere1 "/Game/BP/BP_Motor.BP_Motor_C" :!class /Script/Engine.PrimitiveComponent)) 0) (== (Utilities|Array|Length (Collision|GetOverlappingActors _sphere1 "/Game/BP/BP_Steer.BP_Steer_C" :!class /Script/Engine.PrimitiveComponent)) 0))
    (Variables|Default|SetCanSpawn false)
    (Rendering|Material|SetVectorParameterValue "/Game/BP/ChaosMesh/MPC_Color.MPC_Color" "Color" (Utilities|Struct|MakeLinearColor 1.0 0.0 0.0 1.0) :!class /Script/Engine.KismetMaterialLibrary)))

(event OnComponentEndOverlap(Sphere1)
  (params (OverlappedComponent :type Primitive%20Component%20Object%20Reference) (OtherActor :type Actor%20Object%20Reference) (OtherComp :type Primitive%20Component%20Object%20Reference) (OtherBodyIndex :type Integer))
  (bind _sphere1 (Variables|Default|GetSphere1))
  (Utilities|Casting|CastToBP_Motor OtherActor
    (:then
      _)
    (:CastFailed
      (Utilities|Casting|CastToBP_Steer OtherActor)))
  (if (and (== (Utilities|Array|Length (Collision|GetOverlappingActors _sphere1 "/Game/BP/BP_Motor.BP_Motor_C" :!class /Script/Engine.PrimitiveComponent)) 0) (== (Utilities|Array|Length (Collision|GetOverlappingActors _sphere1 "/Game/BP/BP_Steer.BP_Steer_C" :!class /Script/Engine.PrimitiveComponent)) 0))
    (Variables|Default|SetCanSpawn true)
    (Rendering|Material|SetVectorParameterValue "/Game/BP/ChaosMesh/MPC_Color.MPC_Color" "Color" (Utilities|Struct|MakeLinearColor 0.0 1.0 0.0 1.0) :!class /Script/Engine.KismetMaterialLibrary)))

(event Custom|Init
  (params (NewParam :type BP%20Player%20Object%20Reference))
  (bind _output_get (Variables|Default|SetNew%20Param NewParam))
  (Input|EnableInput (Game|GetPlayerController 0))
  (Variables|Default|SetCore (Variables|/Game/BP/BP_Player.BP_Player_C|GetCore _output_get)))

(event EventTick
  (params (DeltaSeconds :type Float%20%28single-precision%29))
  (bind _returnvalue (Game|GetPlayerController 0))
  (bind _newvar (Variables|Default|GetNewVar))
  (bind _newvar_0 (Variables|Default|GetNewVar_0))
  (bind _worldlocation (Game|Player|ConvertMouseLocationToWorldSpace _returnvalue))
  (for _array_element (Variables|Default|GetCore)
    (Utilities|Map|Add _newvar _array_element (Math|Conversions|ToFloat(Integer) (Math|Float|Truncate (Math|Vector|Distance(Vector) (Transformation|GetWorldLocation _array_element) _worldlocation))))
    (Utilities|Map|Add _newvar_0 (Math|Conversions|ToFloat(Integer) (Math|Float|Truncate (Math|Vector|Distance(Vector) (Transformation|GetWorldLocation _array_element) _worldlocation))) _array_element))
  (bind _values (Utilities|Map|Values _newvar))
  (Transformation|SetActorLocation (Math|Vector|MakeVector (.x (+ (Transformation|GetWorldLocation (.Value (Utilities|Map|Find _newvar_0 (.MinValue (Math|Float|MinOfFloatArray _values))))) (* (Math|Vector|GetRightVector (Math|Rotator|CombineRotators (Math|Rotator|FindLookatRotation (Transformation|GetWorldLocation (.Value (Utilities|Map|Find _newvar_0 (.MinValue (Math|Float|MinOfFloatArray _values))))) _worldlocation) "0.000000,-90.000000,0.000000")) 6e+01))) (.y (+ (Transformation|GetWorldLocation (.Value (Utilities|Map|Find _newvar_0 (.MinValue (Math|Float|MinOfFloatArray _values))))) (* (Math|Vector|GetRightVector (Math|Rotator|CombineRotators (Math|Rotator|FindLookatRotation (Transformation|GetWorldLocation (.Value (Utilities|Map|Find _newvar_0 (.MinValue (Math|Float|MinOfFloatArray _values))))) _worldlocation) "0.000000,-90.000000,0.000000")) 6e+01))) 5e+01) false false))

(event Input|MouseEvents|LeftMouseButton
  (params (Key :type Key%20Structure :default "None"))
  (bind _returnvalue (Transformation|GetActorLocation))
  (:Pressed
    (if (Variables|Default|GetCanSpawn)
      (bind _returnvalue_2 (Game|SpawnActorfromClass "/Game/BP/BP_Bubble.BP_Bubble_C" (Math|Transform|MakeTransform (Math|Vector|MakeVector (.x _returnvalue) (.y _returnvalue) 5e+01) "0, 0, 0" "1.000000,1.000000,1.000000") "Undefined" "MultiplyWithRoot" 0 0))
      (Transformation|AttachComponentToComponent (Variables|/Game/BP/BP_Bubble.BP_Bubble_C|GetCore _returnvalue_2) (.Value (Utilities|Map|Find (Variables|Default|GetNewVar_0) (.MinValue (Math|Float|MinOfFloatArray (stale EventTick _values))))) "None" "KeepWorld" "KeepWorld" "KeepWorld" true)
      (Variables|/Game/BP/BP_Bubble.BP_Bubble_C|SetAttached _returnvalue_2 true)
      (Default|AddBubble (Variables|Default|GetNew%20Param) (Variables|/Game/BP/BP_Bubble.BP_Bubble_C|GetCore _returnvalue_2))
      (bind _asbp_bubble (Utilities|Casting|CastToBP_Bubble (Components|GetOwner (.Value (Utilities|Map|Find (Variables|Default|GetNewVar_0) (.MinValue (Math|Float|MinOfFloatArray (stale EventTick _values))))))))
      (Default|List _asbp_bubble _returnvalue_2)
      (Default|ResetSpawn (Variables|Default|GetNew%20Param))
      (Actor|DestroyActor)
      (Utilities|Map|Clear (Variables|Default|GetNewVar))
      (Utilities|Map|Clear (Variables|Default|GetNewVar_0)))))

(event Input|MouseEvents|RightMouseButton
  (params (Key :type Key%20Structure :default "None"))
  (:Pressed
    (Default|ResetSpawn (Variables|Default|GetNew%20Param))
    (Actor|DestroyActor)))

(fn ConstructionScript)