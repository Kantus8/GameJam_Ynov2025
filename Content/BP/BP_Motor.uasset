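; BP_Motor is a motor actor that pushes its Cube forward with physics and can be sold by clicking.
; Initialisation registers it with the passed-in owner, starts a fast looping timer that applies force along the Cube's forward vector, and plays a timeline that scales the Cube up slightly.
; When clicked while the owner's Delete flag is set, it unregisters, notifies the HUD of the sale and destroys itself.
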(event Custom|CustomEvent
  (bind _cube (Variables|Default|GetCube))
  (Class|PrimitiveComponent|AddForceatLocation _cube (* (Math|Vector|GetForwardVector _cube) 4e+03) (Transformation|GetWorldLocation _cube) "None"))

(event EventInitialisation
  (params (NewParam :type BP%20Player%20Object%20Reference))
  (Utilities|Time|SetTimerbyEvent (delegate Custom|CustomEvent) 0.01 true)
  (Default|AddMotor NewParam)
  (Variables|Default|SetNewVar (Transformation|GetWorldScale (Variables|Default|GetCube)))
  (bind _newtrack_0 (Timeline|Timeline PlayFromStart)
    (:Update
      (Transformation|SetWorldScale3D (Variables|Default|GetCube) (* (Variables|Default|GetNewVar) (Math|Float|Lerp 1.0 1.1 _newtrack_0))))))

(event MouseInput|EventActorOnClicked
  (params (ButtonPressed :type Key%20Structure :default "None"))
  (if (Variables|/Game/BP/BP_Player.BP_Player_C|GetDelete (stale EventInitialisation NewParam))
    (Default|RemoveMotor (stale EventInitialisation NewParam))
    (Default|Sold (Variables|/Game/BP/BP_Player.BP_Player_C|GetHUD (stale EventInitialisation NewParam)))
    (Actor|DestroyActor)))

(fn ConstructionScript)