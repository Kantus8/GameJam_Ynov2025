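; Player actor for a game of building a craft from bubbles and items, handling HUD and menu creation, input and pause.
; Spawns preview actors for bubbles and items behind resettable DoOnce gates, with a delete/sell mode and HUD refunds.
; Each tick it moves to the average position of the Core bubbles and widens the orthographic camera with their count.
; Without motors, input nudges the first core; motor and steer counts govern torque.
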(event Custom|ResetSpawn
  (Utilities|FlowControl|DoOnce false) ; enters at Reset
)

(event Custom|AddBubble
  (params (NewBubbleCore :type Static%20Mesh%20Component%20Object%20Reference))
  (Utilities|Array|Add (Variables|Default|GetCore) NewBubbleCore))

(event Custom|Remove%20Steer
  (Math|Integer|DecrementInt (Variables|Default|GetSteerNumber)))

(event Custom|SpawnBubble
  (if (> (Variables|/Game/BubbleGame/WB_HUD.WB_HUD_C|GetBubbleAmount (stale Custom|StartGame _returnvalue)) 0)
    (Utilities|FlowControl|DoOnce false
      (:Completed
        (Variables|/Game/BubbleGame/WB_HUD.WB_HUD_C|SetBubbleAmount (stale Custom|StartGame _returnvalue) (- (Variables|/Game/BubbleGame/WB_HUD.WB_HUD_C|GetBubbleAmount (stale Custom|StartGame _returnvalue)) 1))
        (Variables|/Game/BubbleGame/WB_HUD.WB_HUD_C|SetBubbleMax (stale Custom|StartGame _returnvalue) false)
        (Variables|Default|SetDelete false)
        (bind _returnvalue (Game|SpawnActorfromClass "/Game/BP/BP_PreviewBubble.BP_PreviewBubble_C" (Math|Transform|MakeTransform "0, 0, 0" "0, 0, 0" "1.000000,1.000000,1.000000") "Undefined" "MultiplyWithRoot" 0 0))
        (Default|Init _returnvalue self)
        (Default|ReseetSell (Variables|Default|GetHUD))))))

(event Custom|SpawnItem
  (params (NewParam :type Actor%20Class%20Reference))
  (Utilities|FlowControl|DoOnce false
    (:Completed
      (Variables|Default|SetDelete false)
      (bind _returnvalue (Game|SpawnActorfromClass "/Game/BP/BP_PreviewMotor.BP_PreviewMotor_C" (Math|Transform|MakeTransform "0, 0, 0" "0, 0, 0" "1.000000,1.000000,1.000000") "Undefined" "MultiplyWithRoot" 0 0))
      (Default|Init _returnvalue self NewParam)
      (Default|ReseetSell (Variables|Default|GetHUD)))))

(event Custom|AddSteer
  (params (NewParam :type BP%20Steer%20Object%20Reference))
  (Math|Integer|IncrementInt (Variables|Default|GetSteerNumber)))

(event Custom|Add%20Motor
  (Math|Integer|IncrementInt (Variables|Default|GetMotorNumber)))

(event Custom|SellItem
  (bind _hud (Variables|Default|GetHUD))
  (Variables|Default|SetDelete true)
  (bind _returnvalue (Actor|GetActorOfClass "/Game/BP/BP_PreviewBubble.BP_PreviewBubble_C"))
  (bind _returnvalue_2 (Actor|GetActorOfClass "/Game/BP/BP_PreviewMotor.BP_PreviewMotor_C"))
  (Utilities|IsValid _returnvalue
    (:Is%20Valid
      (Actor|DestroyActor _returnvalue))
    (:Is%20Not%20Valid
      _))
  (Utilities|IsValid _returnvalue_2
    (:Is%20Valid
      (Actor|DestroyActor _returnvalue_2))
    (:Is%20Not%20Valid
      _))
  (Variables|/Game/BubbleGame/WB_HUD.WB_HUD_C|SetRessources _hud (+ (Variables|/Game/BubbleGame/WB_HUD.WB_HUD_C|GetRessources _hud) (Variables|/Game/BubbleGame/WB_HUD.WB_HUD_C|GetLastBuy _hud)))
  (switch int (Variables|/Game/BubbleGame/WB_HUD.WB_HUD_C|GetLastItemBuy _hud)
    (:0
      (Variables|/Game/BubbleGame/WB_HUD.WB_HUD_C|SetMotorCost _hud (+ (Variables|/Game/BubbleGame/WB_HUD.WB_HUD_C|GetMotorCost _hud) -25)))
    (:1
      (Variables|/Game/BubbleGame/WB_HUD.WB_HUD_C|SetSteerCost _hud (+ (Variables|/Game/BubbleGame/WB_HUD.WB_HUD_C|GetSteerCost _hud) -25)))
    (:2
      (Variables|/Game/BubbleGame/WB_HUD.WB_HUD_C|SetTurretCost _hud (+ (Variables|/Game/BubbleGame/WB_HUD.WB_HUD_C|GetTurretCost _hud) -25)))
    (:3
      (Variables|/Game/BubbleGame/WB_HUD.WB_HUD_C|SetPiqueCost _hud (+ (Variables|/Game/BubbleGame/WB_HUD.WB_HUD_C|GetPiqueCost _hud) -25)))))

(event Custom|StartGame
  (bind _returnvalue (UserInterface|CreateWidget "/Game/BubbleGame/WB_HUD.WB_HUD_C"))
  (UserInterface|Viewport|AddtoViewport _returnvalue 0)
  (Variables|Default|SetHUD _returnvalue)
  (Default|Init _returnvalue self))

(event Custom|ResetSpawnItem
  (bind _hud (Variables|Default|GetHUD))
  (Utilities|FlowControl|Sequence
    (:then_0
      (Utilities|FlowControl|DoOnce false) ; enters at Reset
    )
    (:then_1
      (bind _returnvalue (Actor|GetActorOfClass "/Game/BP/BP_PreviewMotor.BP_PreviewMotor_C"))
      (Utilities|IsValid _returnvalue
        (:Is%20Valid
          (Variables|/Game/BubbleGame/WB_HUD.WB_HUD_C|SetRessources _hud (+ (Variables|/Game/BubbleGame/WB_HUD.WB_HUD_C|GetRessources _hud) (Variables|/Game/BubbleGame/WB_HUD.WB_HUD_C|GetLastBuy _hud)))
          (switch int (Variables|/Game/BubbleGame/WB_HUD.WB_HUD_C|GetLastItemBuy _hud)
            (:0
              (Variables|/Game/BubbleGame/WB_HUD.WB_HUD_C|SetMotorCost _hud (+ (Variables|/Game/BubbleGame/WB_HUD.WB_HUD_C|GetMotorCost _hud) -25)))
            (:1
              (Variables|/Game/BubbleGame/WB_HUD.WB_HUD_C|SetSteerCost _hud (+ (Variables|/Game/BubbleGame/WB_HUD.WB_HUD_C|GetSteerCost _hud) -25)))
            (:2
              (Variables|/Game/BubbleGame/WB_HUD.WB_HUD_C|SetTurretCost _hud (+ (Variables|/Game/BubbleGame/WB_HUD.WB_HUD_C|GetTurretCost _hud) -25)))
            (:3
              (Variables|/Game/BubbleGame/WB_HUD.WB_HUD_C|SetPiqueCost _hud (+ (Variables|/Game/BubbleGame/WB_HUD.WB_HUD_C|GetPiqueCost _hud) -25)))))))))

(event Custom|Remove%20Motor
  (Math|Integer|DecrementInt (Variables|Default|GetMotorNumber)))

(event Input|EnhancedActionEvents|EnhancedInputActionForward
  (params (ActionValue :type Float%20%28double-precision%29) (ElapsedSeconds :type Float%20%28double-precision%29) (TriggeredSeconds :type Float%20%28double-precision%29) (InputAction :type Input%20Action%20Object%20Reference :default "/Game/BP/Input/Forward.Forward"))
  (if (not (> (Variables|Default|GetMotorNumber) 0))
    (Physics|AddImpulse (Utilities|Array|Get(acopy) (Variables|Default|GetCore)) (* (Math|Vector|GetUpVector (Variables|Default|GetCamera)) (* ActionValue 2e+01)) "None" false)))

(event Input|EnhancedActionEvents|EnhancedInputActionRotate
  (params (ActionValue :type Float%20%28double-precision%29) (ElapsedSeconds :type Float%20%28double-precision%29) (TriggeredSeconds :type Float%20%28double-precision%29) (InputAction :type Input%20Action%20Object%20Reference :default "/Game/BP/Input/Rotate.Rotate"))
  (bind _motornumber (Variables|Default|GetMotorNumber))
  (bind _core (Variables|Default|GetCore))
  (bind _returnvalue (> _motornumber 0))
  (for _array_element _core
    (if _returnvalue
      (Class|PrimitiveComponent|AddTorqueinDegrees _array_element (* (* ActionValue 4.5e+06 0.0) (+ (Variables|Default|GetSteerNumber) 1)) "None" false)))
  (if (not _returnvalue)
    (Physics|AddImpulse (Utilities|Array|Get(acopy) _core) (* (Math|Vector|GetRightVector (Variables|Default|GetCamera)) (* ActionValue 2e+01)) "None" false)))

(event EventBeginPlay
  (bind _returnvalue (Game|GetPlayerController 0))
  (bind _returnvalue_2 (Game|GetPlayerController 0))
  (bind _returnvalue_3 (PlayerController|LocalPlayerSubsystems|GetEnhancedInputLocalPlayerSubsystem _returnvalue_2))
  (Variables|/Script/Engine.PlayerController|SetbShowMouseCursor _returnvalue true)
  (Variables|/Script/Engine.PlayerController|SetbEnableClickEvents _returnvalue true)
  (Game|Player|SetViewTargetwithBlend _returnvalue self 0.0 "VTBlend_Linear" 0.0 false)
  (Utilities|IsValid _returnvalue_3
    (:Is%20Valid
      (Input|AddMappingContext _returnvalue_3 "/Game/BP/Input/IMC_Base.IMC_Base" 0 "(bIgnoreAllPressedKeysUntilRelease=True,bForceImmediately=False,bNotifyUserSettings=False)")
      (bind _returnvalue_4 (UserInterface|CreateWidget "/Game/BP/WB_MainMenu.WB_MainMenu_C"))
      (UserInterface|Viewport|AddtoViewport _returnvalue_4 0)
      (Default|InitMENU _returnvalue_4 self))))

(event EventTick
  (params (DeltaSeconds :type Float%20%28single-precision%29))
  (for (_array_element _array_index) (Variables|Default|GetCore)
    (Variables|Default|SetNewVar_0 (+ (Transformation|GetWorldLocation _array_element) (Variables|Default|GetNewVar_0))))
  (bind _output_get (Variables|Default|SetNewVar_0 (/ (Variables|Default|GetNewVar_0) (+ _array_index 1))))
  (Transformation|SetActorLocation _output_get false false)
  (Variables|Default|SetNewVar_0 "0, 0, 0")
  (Class|CameraComponent|SetOrthoWidth (Variables|Default|GetCamera) (Math|Conversions|ToFloat(Integer) (Math|Integer|Clamp(Integer) (+ 1200 (* (Utilities|Array|Length (Variables|Default|GetCore)) 75)) 1000 3000))))

(event Input|MouseEvents|RightMouseButton
  (params (Key :type Key%20Structure :default "None"))
  (:Pressed
    (if (Variables|Default|GetDelete)
      (Variables|Default|SetDelete false)
      (Default|ReseetSell (Variables|Default|GetHUD)))))

(event Input|KeyboardEvents|Escape
  (params (Key :type Key%20Structure :default "None"))
  (:Pressed
    (Utilities|FlowControl|FlipFlop
      (:A
        (Game|SetGamePaused true))
      (:B
        (Game|SetGamePaused false)))))

(event Input|KeyboardEvents|P
  (params (Key :type Key%20Structure :default "None"))
  (:Pressed
    (Utilities|FlowControl|FlipFlop
      (:A
        (Game|SetGamePaused true))
      (:B
        (Game|SetGamePaused false)))))

(fn ConstructionScript)